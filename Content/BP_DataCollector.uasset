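; Data collector Blueprint that records a facade study session: setting changes, task progress, scan and GUI test completion, and head, facade and gaze data.
; When LogActive is set, each Log function appends a delimited string with game time and UTC timestamp to the Logged array and passes it to PrintString.
; HeadDataReadyToLog reports when HeadTransformLogFrequency seconds have elapsed since the last head entry.
; The file shows no saving of Logged to disk.
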(fn `DEPRECATED_GetCurrentTime`
  (returns (CurrentTime :type "Float (double-precision)") (ElapsedTIme :type "Float (double-precision)"))
  (return (`KismetSystemLibrary.GetGameTimeInSeconds`) (- (`KismetSystemLibrary.GetGameTimeInSeconds`) (`self.StartTime`))))

(fn `GetTimeAsString`
  (returns (CurrentTime :type String))
  (bind (_year _month _day _hour _minute _second _millisecond) (`KismetMathLibrary.BreakDateTime` (`KismetMathLibrary.UtcNow`)))
  (return (`KismetStringLibrary.Concat_StrStr` (`KismetStringLibrary.Conv_IntToString` _year) "_" (`KismetStringLibrary.Conv_IntToString` _month) "_" (`KismetStringLibrary.Conv_IntToString` _day) "-" (`KismetStringLibrary.Conv_IntToString` _hour) ":" (`KismetStringLibrary.Conv_IntToString` _minute) ":" (`KismetStringLibrary.Conv_IntToString` _second) "." (`KismetStringLibrary.Conv_IntToString` _millisecond))))

(fn `HeadDataReadyToLog`
  (returns (bReady :type Boolean))
  (if (>= (- (`KismetSystemLibrary.GetGameTimeInSeconds`) (`self.LastHeadLogTime`)) (`self.HeadTransformLogFrequency`))
    (return true)
    (else
      (return false))))

(fn `LogAllTasksComplete`
  (if (`self.bLogActive`)
    (bind _currenttime (`self.GetTimeAsString`))
    (bind _returnvalue (`KismetStringLibrary.Concat_StrStr` " \n==================== \nAll_Tasks_Complete" (`KismetStringLibrary.Concat_StrStr` "" " \nCurrent: \n" (`KismetStringLibrary.Conv_DoubleToString` (`KismetSystemLibrary.GetGameTimeInSeconds`)) " \nTimestamp: \n" _currenttime " \n====================")))
    (`KismetArrayLibrary.Array_Add` (`self.Logged`) _returnvalue)
    (`KismetSystemLibrary.PrintString` _returnvalue (`self.bPrintToScreen`))
    (else
      (return))))

(fn `LogEndTask`
  (params (Task :type "/Game/F_Task Structure"))
  (if (`self.bLogActive`)
    (bind _currenttime (`self.GetTimeAsString`))
    (bind _returnvalue (`KismetStringLibrary.Concat_StrStr` " \n==================== \nEnd_Task" (`KismetStringLibrary.Concat_StrStr` "" " \nCurrent: \n" (`KismetStringLibrary.Conv_DoubleToString` (`KismetSystemLibrary.GetGameTimeInSeconds`)) " \nTimestamp: \n" _currenttime " \n--------------------" " \nEnd_Task: \n" (`.Name_3_1CBA63C14B885B62C66644BBC3CB5C4D` (break `/Game/F_Task` Task)) " \n====================")))
    (`KismetArrayLibrary.Array_Add` (`self.Logged`) _returnvalue)
    (`KismetSystemLibrary.PrintString` _returnvalue (`self.bPrintToScreen`))
    (else
      (return))))

(fn `LogGUITestComplete`
  (if (`self.bLogActive`)
    (bind _currenttime (`self.GetTimeAsString`))
    (bind _returnvalue (`KismetStringLibrary.Concat_StrStr` " \n==================== \nGUI_Test_Complete" (`KismetStringLibrary.Concat_StrStr` "" " \nCurrent: \n" (`KismetStringLibrary.Conv_DoubleToString` (`KismetSystemLibrary.GetGameTimeInSeconds`)) " \nTimestamp: \n" _currenttime " \n====================")))
    (`KismetArrayLibrary.Array_Add` (`self.Logged`) _returnvalue)
    (`KismetSystemLibrary.PrintString` _returnvalue (`self.bPrintToScreen`))
    (else
      (return))))

(fn `LogHeadData`
  (params (HeadPosition :type "Vector Structure") (HeadRotation :type "Rotator Structure") (FacadePosition :type "Vector Structure") (FacadeRotation :type "Rotator Structure") (bValidReading :type Boolean) (GazeOrigin :type "Vector Structure") (GazeDirection :type "Vector Structure") (GazeConfidence :type "Float (double-precision)"))
  (if (`self.bLogActive`)
    (bind _currenttime (`self.GetTimeAsString`))
    (bind _returnvalue (`KismetStringLibrary.Concat_StrStr` " \n==================== \nHead" (`KismetStringLibrary.Concat_StrStr` "" " \nCurrent: \n" (`KismetStringLibrary.Conv_DoubleToString` (`KismetSystemLibrary.GetGameTimeInSeconds`)) " \nTimestamp: \n" _currenttime " \n--------------------") (`KismetStringLibrary.Concat_StrStr` "" " \nHead_Position: \n" (`KismetStringLibrary.Conv_VectorToString` HeadPosition) " \nHead_Rotation: \n" (`KismetStringLibrary.Conv_RotatorToString` HeadRotation) " \nFacade_Position: \n" (`KismetStringLibrary.Conv_VectorToString` FacadePosition) " \nFacade_Rotation: \n" (`KismetStringLibrary.Conv_RotatorToString` FacadeRotation) " \nGaze_Valid: \n" (`KismetStringLibrary.Conv_BoolToString` bValidReading) " \nGaze_Origin: \n" (`KismetStringLibrary.Conv_VectorToString` GazeOrigin) " \nGaze_Direction: \n" (`KismetStringLibrary.Conv_VectorToString` GazeDirection) " \nGaze_Confidence: \n" (`KismetStringLibrary.Conv_DoubleToString` GazeConfidence) " \n====================")))
    (`KismetArrayLibrary.Array_Add` (`self.Logged`) _returnvalue)
    (`KismetSystemLibrary.PrintString` _returnvalue (`self.bPrintToScreen`))
    (set `self.LastHeadLogTime` (`KismetSystemLibrary.GetGameTimeInSeconds`))
    (else
      (return))))

(fn `LogPreviousTask`
  (params (Task :type "/Game/F_Task Structure"))
  (if (`self.bLogActive`)
    (bind _currenttime (`self.GetTimeAsString`))
    (bind _returnvalue (`KismetStringLibrary.Concat_StrStr` " \n==================== \nUndo_Task" (`KismetStringLibrary.Concat_StrStr` "" " \nCurrent: \n" (`KismetStringLibrary.Conv_DoubleToString` (`KismetSystemLibrary.GetGameTimeInSeconds`)) " \nTimestamp: \n" _currenttime " \n--------------------" " \nUndo_Task: \n" (`.Name_3_1CBA63C14B885B62C66644BBC3CB5C4D` (break `/Game/F_Task` Task)) " \n====================")))
    (`KismetArrayLibrary.Array_Add` (`self.Logged`) _returnvalue)
    (`KismetSystemLibrary.PrintString` _returnvalue (`self.bPrintToScreen`))
    (else
      (return))))

(fn `LogScanComplete`
  (if (`self.bLogActive`)
    (bind _currenttime (`self.GetTimeAsString`))
    (bind _returnvalue (`KismetStringLibrary.Concat_StrStr` " \n==================== \nScan_Complete" (`KismetStringLibrary.Concat_StrStr` "" " \nCurrent: \n" (`KismetStringLibrary.Conv_DoubleToString` (`KismetSystemLibrary.GetGameTimeInSeconds`)) " \nTimestamp: \n" _currenttime " \n====================")))
    (`KismetArrayLibrary.Array_Add` (`self.Logged`) _returnvalue)
    (`KismetSystemLibrary.PrintString` _returnvalue (`self.bPrintToScreen`))
    (else
      (return))))

(fn `LogSettingsChanged`
  (params (FacadeSetting :type "/Game/E_FacadeSetting Enum" :default "NewEnumerator0") (TimeSetting :type "/Game/E_TimeSetting Enum" :default "NewEnumerator0") (PositionSetting :type "/Game/E_PositionSetting Enum" :default "NewEnumerator0") (RoomSetting :type "/Game/E_RoomSetting Enum" :default "NewEnumerator0") (bRadiationMapSetting :type Boolean) (bFacadeVisible :type Boolean) (SettingChanged :type String))
  (if (`self.bLogActive`)
    (bind _currenttime (`self.GetTimeAsString`))
    (bind _returnvalue (`KismetStringLibrary.Concat_StrStr` " \n==================== \nSettings_Changed" (`KismetStringLibrary.Concat_StrStr` "" " \nCurrent: \n" (`KismetStringLibrary.Conv_DoubleToString` (`KismetSystemLibrary.GetGameTimeInSeconds`)) " \nTimestamp: \n" _currenttime " \n--------------------") (`KismetStringLibrary.Concat_StrStr` " \nFacade: \n" (`|GetEnumeratorNameAsString` FacadeSetting) " \nPosition: \n" (`|GetEnumeratorNameAsString` PositionSetting) " \nRoom: \n" (`|GetEnumeratorNameAsString` RoomSetting) " \nTime: \n" (`|GetEnumeratorNameAsString` TimeSetting) " \nRadiation: \n" (`KismetStringLibrary.Conv_BoolToString` bRadiationMapSetting) " \nFacade_Visible: \n" (`KismetStringLibrary.Conv_BoolToString` bFacadeVisible) " \nSetting_Changed: \n" SettingChanged " \n====================")))
    (`KismetArrayLibrary.Array_Add` (`self.Logged`) _returnvalue)
    (`KismetSystemLibrary.PrintString` _returnvalue (`self.bPrintToScreen`))
    (else
      (return))))

(fn `LogStartTask`
  (params (Task :type "/Game/F_Task Structure"))
  (if (`self.bLogActive`)
    (bind _currenttime (`self.GetTimeAsString`))
    (bind _returnvalue (`KismetStringLibrary.Concat_StrStr` " \n==================== \nStart_Task" (`KismetStringLibrary.Concat_StrStr` "" " \nCurrent: \n" (`KismetStringLibrary.Conv_DoubleToString` (`KismetSystemLibrary.GetGameTimeInSeconds`)) " \nTimestamp: \n" _currenttime " \n--------------------" " \nStart_Task: \n" (`.Name_3_1CBA63C14B885B62C66644BBC3CB5C4D` (break `/Game/F_Task` Task)) " \n====================")))
    (`KismetArrayLibrary.Array_Add` (`self.Logged`) _returnvalue)
    (`KismetSystemLibrary.PrintString` _returnvalue (`self.bPrintToScreen`))
    (else
      (return))))

(fn `Start`
  (set `self.StartTime` (`KismetSystemLibrary.GetGameTimeInSeconds`)))

(fn `StartTask`
  (params (Task :type "/Game/F_Task Structure"))
  (bind _output_get (set `self.CurrentTask` Task))
  (set `self.TaskStartTime` (`KismetSystemLibrary.GetGameTimeInSeconds`))
  (`self.LogStartTask` _output_get))

(fn `UserConstructionScript`)