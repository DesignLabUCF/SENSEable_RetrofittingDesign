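; Extra simulation menu on a UX Tools hand menu, shown while the right palm-up constraint is active.
; Pressable buttons drive BP_SimController to toggle room and facade visibility, reset, and cycle room, facade and time, and start or stop BP_AudioCapturer recording.
; Controller setting updates refresh the selection labels, while Tick updates the recording timer.
; Hiding also teleports the back plate far away as a collision workaround.
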(event `self.ReceiveBeginPlay`
  (bind _childactor (`ChildActorComponent.ChildActor` (`self.3_Button`)))
  (`self.SetMenuVisibility` false)
  (bind _returnvalue (`GameplayStatics.GetActorOfClass` "/Game/BP_SimController.BP_SimController_C"))
  (bind _output_get (set `self.SimulationController` _returnvalue))
  (add `/Game/BP_SimController.SimulationSettingsUpdated` _output_get (delegate `SimulationSettingUpdated_Event`))
  (bind _returnvalue_2 (`GameplayStatics.GetActorOfClass` "/Game/BP_AudioCapturer.BP_AudioCapturer_C"))
  (set `self.AudioCapturerActor` _returnvalue_2)
  (`|ExecutionSequence`
    (:`then_0`
      (add `UxtPressableButtonComponent.OnButtonPressed` (`self.GetComponentByClass` (`ChildActorComponent.ChildActor` (`self.1_Button`)) "/Script/UXTools.UxtPressableButtonComponent") (delegate `1_Event`)))
    (:`then_1`
      (add `UxtPressableButtonComponent.OnButtonPressed` (`self.GetComponentByClass` (`ChildActorComponent.ChildActor` (`self.2_Button`)) "/Script/UXTools.UxtPressableButtonComponent") (delegate `2_Event`)))
    (:`then_2`
      (add `UxtPressableButtonComponent.OnButtonPressed` (`self.GetComponentByClass` _childactor "/Script/UXTools.UxtPressableButtonComponent") (delegate `Reset_Event`))
      (add `self.OnClicked` _childactor (delegate `OnClicked_Event_6`)))
    (:`then_3`
      (add `UxtPressableButtonComponent.OnButtonPressed` (`self.GetComponentByClass` (`ChildActorComponent.ChildActor` (`self.Room_Button`)) "/Script/UXTools.UxtPressableButtonComponent") (delegate `Room_Event`)))
    (:`then_4`
      (add `UxtPressableButtonComponent.OnButtonPressed` (`self.GetComponentByClass` (`ChildActorComponent.ChildActor` (`self.Facade_Button`)) "/Script/UXTools.UxtPressableButtonComponent") (delegate `Facade_Event`)))
    (:`then_5`
      (add `UxtPressableButtonComponent.OnButtonPressed` (`self.GetComponentByClass` (`ChildActorComponent.ChildActor` (`self.Facade_Button_Back`)) "/Script/UXTools.UxtPressableButtonComponent") (delegate `FacadeBack_Event`)))
    (:`then_6`
      (add `UxtPressableButtonComponent.OnButtonPressed` (`self.GetComponentByClass` (`ChildActorComponent.ChildActor` (`self.Time_Button`)) "/Script/UXTools.UxtPressableButtonComponent") (delegate `Time_Event`)))
    (:`then_7`
      (add `UxtPressableButtonComponent.OnButtonPressed` (`self.GetComponentByClass` (`ChildActorComponent.ChildActor` (`self.StartRecording_Button`)) "/Script/UXTools.UxtPressableButtonComponent") (delegate `StartRecording_Event`)))
    (:`then_8`
      (add `UxtPressableButtonComponent.OnButtonPressed` (`self.GetComponentByClass` (`ChildActorComponent.ChildActor` (`self.StopRecording_Button`)) "/Script/UXTools.UxtPressableButtonComponent") (delegate `EndRecording_Event`)))))

(event `1_Event`
  (params (Button :type "UxtPressableButtonComponent Object Reference") (Pointer :type "UxtPointerComponent Object Reference"))
  (`/Game/BP_SimController.EXTRA_AlternateRoomVisibility` (`self.SimulationController`)))

(event `SimulationSettingUpdated_Event`
  (params (SettingChanged :type String))
  (`self.UpdateGUI`))

(event `2_Event`
  (params (Button :type "UxtPressableButtonComponent Object Reference") (Pointer :type "UxtPointerComponent Object Reference"))
  (`/Game/BP_SimController.EXTRA_AlternateFacadeVisibility` (`self.SimulationController`)))

(event `self.ReceiveTick`
  (params (DeltaSeconds :type "Float (single-precision)"))
  (bind _audiocaptureractor (`self.AudioCapturerActor`))
  (`/Engine/EditorBlueprintResources/StandardMacros.IsValid` _audiocaptureractor
    (:`Is Valid`
      (bind _bactive (`/Game/BP_AudioCapturer.IsCaptureActive` _audiocaptureractor))
      (if _bactive
        (bind _timestring (`/Game/BP_AudioCapturer.GetRecordingTime` (`self.AudioCapturerActor`)))
        (`TextRenderComponent.K2_SetText` (`self.RecordingTime_Text`) (`KismetTextLibrary.Conv_StringToText` _timestring))
        (else
          (`TextRenderComponent.K2_SetText` (`self.RecordingTime_Text`) (`KismetTextLibrary.Conv_StringToText` "00:00.000") :!label _label))))
    (:`Is Not Valid`
      (goto _label))))

(event `OnClicked_Event_6` :!signature `self.OnClicked`
  (params (TouchedActor :type "Actor Object Reference") (ButtonPressed :type "Key Structure" :default "None"))
  (`self.Reset_Event` null))

(event `Reset_Event`
  (params (Button :type "UxtPressableButtonComponent Object Reference") (Pointer :type "UxtPointerComponent Object Reference"))
  (`/Game/BP_SimController.Reset` (`self.SimulationController`)))

(event `self.UxtPalmUpConstraint_Right.OnConstraintActivated`
  (`self.SetMenuVisibility` false))

(event `self.UxtPalmUpConstraint_Right.OnConstraintDeactivated`
  (`self.SetMenuVisibility` true))

(event `Room_Event`
  (params (Button :type "UxtPressableButtonComponent Object Reference") (Pointer :type "UxtPointerComponent Object Reference"))
  (`/Game/BP_SimController.SetRoom` (`self.SimulationController`) true "NewEnumerator0" true true false))

(event `Facade_Event`
  (params (Button :type "UxtPressableButtonComponent Object Reference") (Pointer :type "UxtPointerComponent Object Reference"))
  (`/Game/BP_SimController.SetFacade` (`self.SimulationController`) true "NewEnumerator0" true))

(event `FacadeBack_Event`
  (params (Button :type "UxtPressableButtonComponent Object Reference") (Pointer :type "UxtPointerComponent Object Reference"))
  (`/Game/BP_SimController.SetFacade` (`self.SimulationController`) true "NewEnumerator0" false))

(event `Time_Event`
  (params (Button :type "UxtPressableButtonComponent Object Reference") (Pointer :type "UxtPointerComponent Object Reference"))
  (`/Game/BP_SimController.SetTime` (`self.SimulationController`) true "NewEnumerator0" true))

(event `StartRecording_Event`
  (params (Button :type "UxtPressableButtonComponent Object Reference") (Pointer :type "UxtPointerComponent Object Reference"))
  (`/Game/BP_AudioCapturer.StartCapture` (`self.AudioCapturerActor`)))

(event `EndRecording_Event`
  (params (Button :type "UxtPressableButtonComponent Object Reference") (Pointer :type "UxtPointerComponent Object Reference"))
  (`/Game/BP_AudioCapturer.EndCapture` (`self.AudioCapturerActor`)))

(fn `SetMenuVisibility`
  (params (bHide :type Boolean))
  ;[1 1 1] Visibility
  (`SceneComponent.SetHiddenInGame` (`self.UxtBackPlate`) bHide true)
  ;[1 1 1] Collision
  (if bHide
    (`SceneComponent.K2_SetWorldLocation` (`self.UxtBackPlate`) (-100000.0 0.0 0.0) false true)))

(fn `UpdateGUI`
  (`|ExecutionSequence`
    (:`then_0`
      (`TextRenderComponent.K2_SetText` (`self.Room_Text`) (`KismetTextLibrary.Conv_StringToText` (`|GetEnumeratorNameAsString` (`/Game/BP_SimController.ActiveRoom` (`self.SimulationController`))))))
    (:`then_1`
      (`TextRenderComponent.K2_SetText` (`self.Facade_Text`) (`KismetTextLibrary.Conv_StringToText` (`|GetEnumeratorNameAsString` (`/Game/BP_SimController.ActiveFacade` (`self.SimulationController`))))))
    (:`then_2`
      (`TextRenderComponent.K2_SetText` (`self.Time_Text`) (`KismetTextLibrary.Conv_StringToText` (`|GetEnumeratorNameAsString` (`/Game/BP_SimController.ActiveTime` (`self.SimulationController`))))))))

(fn `UserConstructionScript`)