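; Room controller that cycles through Datasmith-imported rooms and moves a facade between each room's window positions.
; After a short delay for facade setup, it collects scene actors matching RoomNames and toggles visibility recursively through attached actors.
; Room and position changes drive BP_FacadeController's size and transform and fire update notifications.
; Sizes, window transforms and QR-pose-relative offsets are hard-coded for two rooms: conference room and Joe's office.
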(event `self.ReceiveBeginPlay`
  (bind _returnvalue (`GameplayStatics.GetActorOfClass` "/Game/LEGACY/BP_FacadeController.BP_FacadeController_C"))
  (set `self.FacadeController` _returnvalue)
  ;[1 1 1 1 12] Account for Facades not being set yet (TODO better solution
  (`KismetSystemLibrary.Delay` 0.5)
  ;[1 1 1] Set rooms
  (bind _outactors (`GameplayStatics.GetAllActorsOfClass` "/Script/DatasmithContent.DatasmithSceneActor"))
  (for _array_element _outactors
    (bind _bisroom (`self.DatasmithActorIsRoom` _array_element))
    (if _bisroom
      (`KismetArrayLibrary.Array_Add` (`self.Rooms`) _array_element)))
  (`self.HideAllRooms`)
  (`self.SetActiveRoom` (`|GetArrayItem` (`self.Rooms`))))

(fn `ChangePosition`
  (params (bForward :type Boolean))
  (locals (ActiveRoomTransforms :type "Array of Transform Structure"))
  (bind _positioncounter (`self.PositionCounter`))
  (bind _activeroomtransforms (`self.GetActiveRoomTransforms`))
  (if bForward
    (bind _result (`/Engine/EditorBlueprintResources/StandardMacros.IncrementInt` _positioncounter)
      (:`  `
        (bind _returnvalue (- (`KismetArrayLibrary.Array_Length` _activeroomtransforms) 1))
        (if (> _result _returnvalue)
          (set `self.PositionCounter` 0))))
    (else
      (bind _result_2 (`/Engine/EditorBlueprintResources/StandardMacros.DecrementInt` _positioncounter)
        (:`  `
          (if (< _result_2 0)
            (set `self.PositionCounter` _returnvalue))))))
  (`/Game/LEGACY/BP_FacadeController.SetFacadePositionAndRotation` (`self.FacadeController`) (`|GetArrayItem` _activeroomtransforms (`self.PositionCounter`)))
  (`self.ActivePositionUpdated`))

(fn `ChangeRoom`
  (params (bForward :type Boolean))
  (bind _roomcounter (`self.RoomCounter`))
  (bind _returnvalue (- (`KismetArrayLibrary.Array_Length` (`self.Rooms`)) 1))
  (if bForward
    (bind _result (`/Engine/EditorBlueprintResources/StandardMacros.IncrementInt` _roomcounter)
      (:`  `
        (if (> _result _returnvalue)
          (set `self.RoomCounter` 0))))
    (else
      (bind _result_2 (`/Engine/EditorBlueprintResources/StandardMacros.DecrementInt` _roomcounter)
        (:`  `
          (if (< _result_2 0)
            (set `self.RoomCounter` _returnvalue))))))
  (`self.SetActiveRoom` (`|GetArrayItem` (`self.Rooms`) (`self.RoomCounter`))))

(fn `DatasmithActorIsRoom`
  (params (DatasmithActor :type "DatasmithSceneActor Object Reference"))
  (returns (bIsRoom :type Boolean))
  (for _array_element (`self.RoomNames`)
    (if (`KismetStringLibrary.EqualEqual_StrStr` (`KismetSystemLibrary.GetDisplayName` DatasmithActor) _array_element)
      (return true)))
  (return false))

(fn `GetActiveRoomOffsetTransform`
  (params (QRPosition :type "Vector Structure") (QRRotation :type "Rotator Structure"))
  (returns (OffsetTransform :type "Transform Structure"))
  (bind _activeroom (`self.ActiveRoom`))
  (bind _rooms (`self.Rooms`))
  (if (== _activeroom (`|GetArrayItem` _rooms))
    (return (`KismetMathLibrary.MakeTransform` (+ QRPosition (* (`KismetMathLibrary.GetForwardVector` QRRotation) 332.589966) (* (`KismetMathLibrary.NegateVector` (`KismetMathLibrary.GetRightVector` QRRotation)) 540.173828) (* (`KismetMathLibrary.GetUpVector` QRRotation) 163.830002)) (`KismetMathLibrary.MakeRotator` (+ (.roll QRRotation) 180.0) (.pitch QRRotation) (+ (.yaw QRRotation) 180.0))))
    (else
      (if (== _activeroom (`|GetArrayItem` _rooms 1))
        _
        (else
          _))
      (return (`KismetMathLibrary.MakeTransform` (+ QRPosition (* (`KismetMathLibrary.GetRightVector` QRRotation) 116.399002) (* (`KismetMathLibrary.GetForwardVector` QRRotation) 439.791656) (* (`KismetMathLibrary.GetUpVector` QRRotation) 163.830002)) (`KismetMathLibrary.MakeRotator` (+ (.roll QRRotation) 180.0) (.pitch QRRotation) (+ (.yaw QRRotation) 90.0)))))))

(fn `GetActiveRoomTransforms`
  (returns (ActiveRoomTransforms :type "Array of Transform Structure"))
  (bind _rooms (`self.Rooms`))
  (bind _activeroom (`self.ActiveRoom`))
  (if (== _activeroom (`|GetArrayItem` _rooms))
    (return (`self.ConfRoomWindowTransforms`))
    (else
      (if (== _activeroom (`|GetArrayItem` _rooms 1))
        _
        (else
          _))
      (return (`self.JoeOfficeWindowTransforms`)))))

(fn `HideAllRooms`
  (for _array_element (`self.Rooms`)
    (`self.HideRoom` _array_element)))

(fn `HideRoom`
  (params (Room :type "Actor Object Reference"))
  (`self.SetActorHiddenInGame` Room true)
  (for _array_element (`self.GetAttachedActors` Room true)
    (`self.HideRoom` _array_element)))

(fn `SetActiveRoom`
  (params (Room :type "DatasmithSceneActor Object Reference"))
  (bind _facadecontroller (`self.FacadeController`))
  (bind _rooms (`self.Rooms`))
  (`self.HideAllRooms`)
  (if (== Room (`|GetArrayItem` _rooms))
    (`/Game/LEGACY/BP_FacadeController.SetFacadeDimensions` _facadecontroller 2.743 3.31)
    (else
      (if (== Room (`|GetArrayItem` _rooms 1))
        _
        (else
          _))
      (`/Game/LEGACY/BP_FacadeController.SetFacadeDimensions` _facadecontroller 2.743 3.8354)))
  (`self.ShowRoom` Room)
  (set `self.ActiveRoom` Room)
  (`self.ActiveRoomUpdated`)
  (`self.SetPosition` 0))

(fn `SetPosition`
  (params (`0` :type Integer))
  (locals (ActiveRoomTransforms :type "Array of Transform Structure"))
  (bind _activeroomtransforms (`self.GetActiveRoomTransforms`))
  (set `self.PositionCounter` `0`)
  (`/Game/LEGACY/BP_FacadeController.SetFacadePositionAndRotation` (`self.FacadeController`) (`|GetArrayItem` _activeroomtransforms (`self.PositionCounter`)))
  (`self.ActivePositionUpdated`))

(fn `ShowConf`
  (`self.ShowRoom` (`|GetArrayItem` (`self.Rooms`))))

(fn `ShowRoom`
  (params (Room :type "Actor Object Reference"))
  (`self.SetActorHiddenInGame` Room false)
  (for _array_element (`self.GetAttachedActors` Room true)
    (`self.ShowRoom` _array_element)))

(fn `UserConstructionScript`)