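; BP_RoomMenu is a palm-up hand menu built with UXT for switching rooms and positions within a room.
; Its pressable buttons call ChangeRoom and ChangePosition on the BP_RoomController found at BeginPlay.
; Controller update events refresh the active room name and position counter text.
; The palm-up constraint shows or hides the back plate, teleporting it far away when hidden, apparently to avoid collision.
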(event `self.ReceiveBeginPlay`
  ;[1 1 1] Init
  (`self.SetMenuVisbility` false)
  (bind _returnvalue (`GameplayStatics.GetActorOfClass` "/Game/LEGACY/BP_RoomController.BP_RoomController_C"))
  (bind _output_get (set `self.RoomController` _returnvalue))
  (add `/Game/LEGACY/BP_RoomController.ActiveRoomUpdated` _output_get (delegate `RoomUpdated_Event`))
  (add `/Game/LEGACY/BP_RoomController.ActivePositionUpdated` _output_get (delegate `PositionUpdated_Event`))
  ;[1 1 1] Buttons (Room)
  (add `UxtPressableButtonComponent.OnButtonPressed` (`self.GetComponentByClass` (`ChildActorComponent.ChildActor` (`self.Button_ForwardRoom`)) "/Script/UXTools.UxtPressableButtonComponent") (delegate `ForwardRoom_Event`))
  (add `UxtPressableButtonComponent.OnButtonPressed` (`self.GetComponentByClass` (`ChildActorComponent.ChildActor` (`self.Button_BackRoom`)) "/Script/UXTools.UxtPressableButtonComponent") (delegate `BackRoom_Event`))
  ;[1 1 1] Buttons (Position)
  (add `UxtPressableButtonComponent.OnButtonPressed` (`self.GetComponentByClass` (`ChildActorComponent.ChildActor` (`self.Button_ForwardPosition`)) "/Script/UXTools.UxtPressableButtonComponent") (delegate `ForwardPosition_Event`))
  (add `UxtPressableButtonComponent.OnButtonPressed` (`self.GetComponentByClass` (`ChildActorComponent.ChildActor` (`self.Button_BackPosition`)) "/Script/UXTools.UxtPressableButtonComponent") (delegate `BackPosition_Event`)))

(event `ForwardRoom_Event`
  (params (Button :type "UxtPressableButtonComponent Object Reference") (Pointer :type "UxtPointerComponent Object Reference"))
  ;[1 1 1] Buttons (Room)
  (`/Game/LEGACY/BP_RoomController.ChangeRoom` (`self.RoomController`) true))

(event `RoomUpdated_Event`
  ;[1 1 1] Init
  (`self.UpdateRoomText`))

(event `BackRoom_Event`
  (params (Button :type "UxtPressableButtonComponent Object Reference") (Pointer :type "UxtPointerComponent Object Reference"))
  ;[1 1 1] Buttons (Room)
  (`/Game/LEGACY/BP_RoomController.ChangeRoom` (`self.RoomController`) false))

(event `PositionUpdated_Event`
  ;[1 1 1] Init
  (`self.UpdatePositionText`))

(event `ForwardPosition_Event`
  (params (Button :type "UxtPressableButtonComponent Object Reference") (Pointer :type "UxtPointerComponent Object Reference"))
  ;[1 1 1] Buttons (Position)
  (`/Game/LEGACY/BP_RoomController.ChangePosition` (`self.RoomController`) true))

(event `self.UxtPalmUpConstraint.OnConstraintActivated`
  (`self.UpdateRoomText`)
  (`self.SetMenuVisbility` false))

(event `BackPosition_Event`
  (params (Button :type "UxtPressableButtonComponent Object Reference") (Pointer :type "UxtPointerComponent Object Reference"))
  ;[1 1 1] Buttons (Position)
  (`/Game/LEGACY/BP_RoomController.ChangePosition` (`self.RoomController`) false))

(event `self.UxtPalmUpConstraint.OnConstraintDeactivated`
  (`self.SetMenuVisbility` true))

(fn `SetMenuVisbility`
  (params (bHide :type Boolean))
  ;[1 1 1] Visibility
  (`SceneComponent.SetHiddenInGame` (`self.UxtBackPlate`) bHide true)
  ;[1 1 1] Collision
  (if bHide
    (`SceneComponent.K2_SetWorldLocation` (`self.UxtBackPlate`) (-100000.0 0.0 0.0) false true)))

(fn `UpdatePositionText`
  (bind _roomcontroller (`self.RoomController`))
  (bind _activeroomtransforms (`/Game/LEGACY/BP_RoomController.GetActiveRoomTransforms` _roomcontroller))
  (`TextRenderComponent.K2_SetText` (`self.Text_Position`) (`KismetTextLibrary.Conv_StringToText` (`KismetStringLibrary.Concat_StrStr` "Position " (`KismetStringLibrary.Conv_IntToString` (+ (`/Game/LEGACY/BP_RoomController.PositionCounter` _roomcontroller) 1)) " of " (`KismetStringLibrary.Conv_IntToString` (`KismetArrayLibrary.Array_Length` _activeroomtransforms))))))

(fn `UpdateRoomText`
  (`TextRenderComponent.K2_SetText` (`self.Text_Facade`) (`KismetTextLibrary.Conv_StringToText` (`KismetSystemLibrary.GetDisplayName` (`/Game/LEGACY/BP_RoomController.ActiveRoom` (`self.RoomController`))))))

(fn `UserConstructionScript`)