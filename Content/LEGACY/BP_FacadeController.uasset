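; AR facade controller that cycles through Datasmith-imported building facades, showing one at a time.
; On BeginPlay it collects keyword-named DatasmithSceneActors, applies M_Facade to their meshes and shows the first.
; Tracked QR-code updates reposition the controller through BP_RoomController's active-room offset.
; Functions switch facades with wraparound, set glass opacity, and forward size and placement changes to facades and BP_Glass; holding P temporarily raises glass opacity.
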(event `self.ReceiveBeginPlay`
  (bind _returnvalue (`GameplayStatics.GetActorOfClass` "/Game/BP_Glass.BP_Glass_C"))
  (set `self.WindowV` _returnvalue)
  (bind _returnvalue_2 (`GameplayStatics.GetActorOfClass` "/Game/LEGACY/BP_RoomController.BP_RoomController_C"))
  (set `self.RoomController` _returnvalue_2)
  ;[1 1 1] Set facades
  (bind _outactors (`GameplayStatics.GetAllActorsOfClass` "/Script/DatasmithContent.DatasmithSceneActor"))
  (for _array_element _outactors
    (bind _bisfacade (`self.DatasmithActorIsFacade` _array_element))
    (if _bisfacade
      (`KismetArrayLibrary.Array_Add` (`self.Facades`) _array_element)))
  (`self.SetTwoSidedMaterial`)
  (`self.HideAllFacades`)
  (`self.SetActiveFacade` (`|GetArrayItem` (`self.Facades`))))

(event `Key|P`
  (params (Key :type "Key Structure"))
  (:`Pressed`
    (`MaterialInstanceDynamic.SetScalarParameterValue` (`self.WindowMaterial`) "Opacity_Param" 0.75))
  (:`Released`
    (`MaterialInstanceDynamic.SetScalarParameterValue` (`self.WindowMaterial`) "Opacity_Param" 0.1)))

(event `self.ARTrackableNotify.OnUpdateTrackedImage`
  (params (TrackedImage :type "ARTrackedImage Object Reference"))
  (bind _asartracked_qrcode (cast `ARTrackedQRCode` TrackedImage))
  (bind (_returnvalue_location _returnvalue_rotation) (`KismetMathLibrary.BreakTransform` (`ARTrackedGeometry.GetLocalToWorldTransform` _asartracked_qrcode)))
  (bind _offsettransform (`/Game/LEGACY/BP_RoomController.GetActiveRoomOffsetTransform` (`self.RoomController`) _returnvalue_location _returnvalue_rotation))
  (`self.K2_SetActorTransform` (`KismetMathLibrary.MakeTransform` (.location _offsettransform) (.rotation _offsettransform))))

(fn `ChangeFacade`
  (params (bForward :type Boolean))
  (bind _facadecounter (`self.FacadeCounter`))
  (bind _returnvalue (- (`KismetArrayLibrary.Array_Length` (`self.Facades`)) 1))
  (if bForward
    (bind _result (`/Engine/EditorBlueprintResources/StandardMacros.IncrementInt` _facadecounter)
      (:`  `
        (if (> _result _returnvalue)
          (set `self.FacadeCounter` 0))))
    (else
      (bind _result_2 (`/Engine/EditorBlueprintResources/StandardMacros.DecrementInt` _facadecounter)
        (:`  `
          (if (< _result_2 0)
            (set `self.FacadeCounter` _returnvalue))))))
  (`self.SetActiveFacade` (`|GetArrayItem` (`self.Facades`) (`self.FacadeCounter`))))

(fn `DatasmithActorIsFacade`
  (params (DatasmithActor :type "DatasmithSceneActor Object Reference"))
  (returns (bIsFacade :type Boolean))
  (for _array_element (`self.FacadeKeywords`)
    (if (`KismetStringLibrary.Contains` (`KismetSystemLibrary.GetDisplayName` DatasmithActor) _array_element)
      (return true)))
  (return false))

(fn `GetDatasmithActorMeshes`
  (params (DatasmithSceneActor :type "DatasmithSceneActor Object Reference"))
  (returns (StaticMeshActors :type "Array of Actor Object Reference"))
  (locals (Actors :type "Array of Actor Object Reference"))
  (for _array_element (`self.GetAttachedActors` DatasmithSceneActor true)
    (`KismetArrayLibrary.Array_Append` (`local.Actors`) (`self.GetAttachedActors` _array_element true)))
  (return (`local.Actors`)))

(fn `HideAllFacades`
  (for _array_element (`self.Facades`)
    (bind _staticmeshactors (`self.GetDatasmithActorMeshes` _array_element))
    (for _array_element_2 _staticmeshactors
      (`self.SetActorHiddenInGame` _array_element_2 true))))

(fn `SetActiveFacade`
  (params (Facade :type "DatasmithSceneActor Object Reference"))
  (`self.HideAllFacades`)
  (bind _staticmeshactors (`self.GetDatasmithActorMeshes` Facade))
  (for _array_element _staticmeshactors
    (`self.SetActorHiddenInGame` _array_element false))
  (set `self.ActiveFacade` Facade)
  (`self.ActiveFacadeUpdated`)
  (`KismetSystemLibrary.PrintString` (`KismetStringLibrary.Concat_StrStr` "Facade Set: " (`KismetSystemLibrary.GetDisplayName` Facade))))

(fn `SetFacadeDimensions`
  (params (Height :type "Float (double-precision)") (Width :type "Float (double-precision)"))
  (for _array_element (`self.Facades`)
    (`self.SetActorScale3D` _array_element (`KismetMathLibrary.MakeVector` Width 1.0 Height)))
  (`/Game/BP_Glass.SetWindowDimensions` (`self.WindowV`) Height Width))

(fn `SetFacadePositionAndRotation`
  (params (Transform :type "Transform Structure"))
  (for _array_element (`self.Facades`)
    (`self.K2_SetActorRelativeLocation` _array_element (.location Transform) false true)
    (`self.K2_SetActorRelativeRotation` _array_element (.rotation Transform) false true)
    (`/Game/BP_Glass.SetWindowPositionAndRotation` (`self.WindowV`) Transform)))

(fn `SetGlassOpacity`
  (params (Opacity :type "Float (double-precision)"))
  (`MaterialInstanceDynamic.SetScalarParameterValue` (`self.WindowMaterial`) "Opacity_Param" Opacity))

(fn `SetTwoSidedMaterial`
  (for _array_element (`self.Facades`)
    (bind _staticmeshactors (`self.GetDatasmithActorMeshes` _array_element))
    (for _array_element_2 _staticmeshactors
      (bind _asstatic_mesh_actor (cast `StaticMeshActor` _array_element_2))
      (`PrimitiveComponent.SetMaterial` (`self.GetComponentByClass` _asstatic_mesh_actor "/Script/Engine.StaticMeshComponent") 0 "/Game/Facades/M_Facade.M_Facade"))))

(fn `UserConstructionScript`)