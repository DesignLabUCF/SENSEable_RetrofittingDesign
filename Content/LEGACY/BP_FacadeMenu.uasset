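; BP_FacadeMenu is a mixed-reality UXT palm-up hand menu for switching building facades and adjusting sun time and glass opacity.
; Forward and back buttons drive BP_FacadeController, whose update event refreshes the facade name label.
; Hour and minute sliders update BP_SunPosition, while the opacity slider feeds BP_Glass.
; The palm-up constraint toggles visibility, and hiding also teleports the backplate far away as a collision workaround.
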(event `self.ReceiveBeginPlay`
  ;[1 1 1] Init
  (`self.SetMenuVisbility` false)
  (bind _returnvalue (`GameplayStatics.GetActorOfClass` "/Game/LEGACY/BP_FacadeController.BP_FacadeController_C"))
  (bind _output_get (set `self.FacadeController` _returnvalue))
  (add `/Game/LEGACY/BP_FacadeController.ActiveFacadeUpdated` _output_get (delegate `ActiveFacadeUpdated_Event`))
  (bind _returnvalue_2 (`GameplayStatics.GetActorOfClass` "/Game/BP_Glass.BP_Glass_C"))
  (set `self.Window` _returnvalue_2)
  ;[1 1 1] Buttons
  (add `UxtPressableButtonComponent.OnButtonPressed` (`self.GetComponentByClass` (`ChildActorComponent.ChildActor` (`self.Button_Forward`)) "/Script/UXTools.UxtPressableButtonComponent") (delegate `Forward_Event`))
  (add `UxtPressableButtonComponent.OnButtonPressed` (`self.GetComponentByClass` (`ChildActorComponent.ChildActor` (`self.Button_Back`)) "/Script/UXTools.UxtPressableButtonComponent") (delegate `Back_Event`))
  ;[1 1 1] Sliders
  (add `UxtPinchSliderComponent.OnUpdateValue` (`self.GetComponentByClass` (`ChildActorComponent.ChildActor` (`self.Slider_Hour`)) "/Script/UXTools.UxtPinchSliderComponent") (delegate `UpdateTime_Event`))
  (add `UxtPinchSliderComponent.OnUpdateValue` (`self.GetComponentByClass` (`ChildActorComponent.ChildActor` (`self.Slider_Minute`)) "/Script/UXTools.UxtPinchSliderComponent") (delegate `UpdateTime_Event`))
  (add `UxtPinchSliderComponent.OnUpdateValue` (`self.GetComponentByClass` (`ChildActorComponent.ChildActor` (`self.Slider_Opacity`)) "/Script/UXTools.UxtPinchSliderComponent") (delegate `UpdateGlass_Event`)))

(event `Forward_Event`
  (params (Button :type "UxtPressableButtonComponent Object Reference") (Pointer :type "UxtPointerComponent Object Reference"))
  ;[1 1 1] Buttons
  (`/Game/LEGACY/BP_FacadeController.ChangeFacade` (`self.FacadeController`) true))

(event `UpdateTime_Event`
  (params (Slider :type "UxtPinchSliderComponent Object Reference") (NewValue :type "Float (double-precision)"))
  ;[1 1 1] Sliders
  (`self.SetTime`))

(event `ActiveFacadeUpdated_Event`
  ;[1 1 1] Init
  (`self.UpdateFacadeText`))

(event `Back_Event`
  (params (Button :type "UxtPressableButtonComponent Object Reference") (Pointer :type "UxtPointerComponent Object Reference"))
  ;[1 1 1] Buttons
  (`/Game/LEGACY/BP_FacadeController.ChangeFacade` (`self.FacadeController`) false))

(event `UpdateGlass_Event`
  (params (Slider :type "UxtPinchSliderComponent Object Reference") (NewValue :type "Float (double-precision)"))
  ;[1 1 1] Sliders
  (`/Game/BP_Glass.SetGlassOpacity` (`self.Window`) NewValue))

(event `self.UxtPalmUpConstraint.OnConstraintActivated`
  (`self.UpdateFacadeText`)
  (`self.SetMenuVisbility` false))

(event `self.UxtPalmUpConstraint.OnConstraintDeactivated`
  (`self.SetMenuVisbility` true))

(fn `SetMenuVisbility`
  (params (bHide :type Boolean))
  ;[1 1 1] Visibility
  (`SceneComponent.SetHiddenInGame` (`self.UxtBackPlate`) bHide true)
  ;[1 1 1] Collision
  (if bHide
    (`SceneComponent.K2_SetWorldLocation` (`self.UxtBackPlate`) (-100000.0 0.0 0.0) false true)))

(fn `SetTime`
  (bind _returnvalue (`GameplayStatics.GetActorOfClass` "/SunPosition/BP_SunPosition.BP_SunPosition_C"))
  (set `/SunPosition/BP_SunPosition.Minutes` (`KismetMathLibrary.Round` (* (`UxtPinchSliderComponent.Value` (`self.GetComponentByClass` (`ChildActorComponent.ChildActor` (`self.Slider_Minute`)) "/Script/UXTools.UxtPinchSliderComponent")) 59.0)) _returnvalue)
  (set `/SunPosition/BP_SunPosition.Hours` (`KismetMathLibrary.Round` (* (`UxtPinchSliderComponent.Value` (`self.GetComponentByClass` (`ChildActorComponent.ChildActor` (`self.Slider_Hour`)) "/Script/UXTools.UxtPinchSliderComponent")) 23.0)) _returnvalue)
  (`/SunPosition/BP_SunPosition.UpdateSun` _returnvalue))

(fn `UpdateFacadeText`
  (`TextRenderComponent.K2_SetText` (`self.Text_Facade`) (`KismetTextLibrary.Conv_StringToText` (`KismetSystemLibrary.GetObjectName` (`/Game/LEGACY/BP_FacadeController.ActiveFacade` (`self.FacadeController`))))))

(fn `UserConstructionScript`)