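; BP_AudioCapturer is a Blueprint that records captured audio to timestamped WAV files.
; StartCapture activates the AudioCapture component, starts recording a submix output and stores the start time, guarded by an Active flag.
; EndCapture deactivates capture and exports the recording, named from the current date and time.
; Helper functions report whether capture is active and the elapsed recording time as a minutes:seconds.milliseconds string.
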(fn `EndCapture`
  (bind (_year _month _day _hour _minute _second) (`KismetMathLibrary.BreakDateTime` (`KismetMathLibrary.Now`)))
  (if (`self.bActive`)
    (set `self.bActive` false)
    (`ActorComponent.Deactivate` (`self.AudioCapture`))
    (`AudioMixerBlueprintLibrary.StopRecordingOutput` "WavFile" (`KismetStringLibrary.Concat_StrStr` (`KismetStringLibrary.Conv_IntToString` _year) "_" (`KismetStringLibrary.Conv_IntToString` _month) "_" (`KismetStringLibrary.Conv_IntToString` _day) "_" (`KismetStringLibrary.Conv_IntToString` _hour) "_" (`KismetStringLibrary.Conv_IntToString` _minute) "_" (`KismetStringLibrary.Conv_IntToString` _second)) "" (`self.Submix`) null)
    (else
      (return))))

(fn `GetRecordingTime`
  (returns (TimeString :type String))
  (bind (_days _hours _minutes _seconds _milliseconds) (`KismetMathLibrary.BreakTimespan` (- (`KismetMathLibrary.Now`) (`self.RecordingStartTime`))))
  (return (`KismetStringLibrary.Concat_StrStr` (`KismetStringLibrary.Conv_IntToString` _minutes) ":" (`KismetStringLibrary.Conv_IntToString` _seconds) "." (`KismetStringLibrary.Conv_IntToString` _milliseconds))))

(fn `IsCaptureActive`
  (returns (bActive :type Boolean))
  (return (`self.bActive`)))

(fn `StartCapture`
  (if (`self.bActive`)
    (return)
    (else
      (set `self.bActive` true)
      (`ActorComponent.Activate` (`self.AudioCapture`) false)
      (`AudioMixerBlueprintLibrary.StartRecordingOutput` 0.0 (`self.Submix`))
      (set `self.RecordingStartTime` (`KismetMathLibrary.Now`)))))

(fn `UserConstructionScript`)