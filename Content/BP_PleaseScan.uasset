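; Actor that displays a world-space "please scan" prompt through a WBP_PleaseScan widget component, with shadow casting off.
; The first ScanComplete switches the widget to a GUI test state, and later completions hide the actor.
; GUITestPassed resets the widget to the scan prompt, in case a rescan is needed, and hides the actor.
; Show and Hide toggle actor visibility and are also bound to G and H debug keys.
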(event `self.ReceiveBeginPlay`
  (`PrimitiveComponent.SetCastShadow` (`self.PleaseScanWidget`) false))

(event `Key|G` :consume false
  (params (Key :type "Key Structure"))
  (:`Pressed`
    (`self.Show`)
    (`KismetSystemLibrary.PrintString` "G")))

(event `Key|H` :consume false
  (params (Key :type "Key Structure"))
  (:`Pressed`
    (`self.Hide`)
    (`KismetSystemLibrary.PrintString` "H")))

(fn `GUITestPassed`
  (bind _aswbp_please_scan (cast `/Game/WBP_PleaseScan` (`WidgetComponent.GetUserWidgetObject` (`self.PleaseScanWidget`))))
  (`/Game/WBP_PleaseScan.SetToPleaseScan` _aswbp_please_scan) ; Set to indicate a rescan is needed in case original scan is reset
  (`self.Hide`))

(fn `Hide`
  (`self.SetActorHiddenInGame` true))

(fn `ScanComplete`
  (if (`self.b_InitialScanComplete`)
    (`self.Hide`)
    (else
      (bind _aswbp_please_scan (cast `/Game/WBP_PleaseScan` (`WidgetComponent.GetUserWidgetObject` (`self.PleaseScanWidget`))))
      (`/Game/WBP_PleaseScan.SetToGUITest` _aswbp_please_scan)
      (set `self.b_InitialScanComplete` true))))

(fn `Show`
  (`self.SetActorHiddenInGame` false))

(fn `UserConstructionScript`)