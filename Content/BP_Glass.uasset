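; BP_Glass is a glass window actor whose opacity, size and placement are set through its functions.
; BeginPlay creates a dynamic instance of M_Glass on the Window component, and SetGlassOpacity drives its Opacity_Param.
; SetWindowDimensions scales the mesh in world space from height and width, multiplied by 100.
; SetWindowPositionAndRotation teleports the actor to a given relative transform with a small Y offset and 90-degree roll and pitch corrections.
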(event `self.ReceiveBeginPlay`
  (bind _returnvalue (`KismetMaterialLibrary.CreateDynamicMaterialInstance` "/Game/Facades/M_Glass.M_Glass" "M_Window_Instance"))
  (bind _output_get (set `self.WindowMaterial` _returnvalue))
  (`PrimitiveComponent.SetMaterial` (`self.window`) 0 _output_get))

(fn `SetGlassOpacity`
  (params (Opacity :type "Float (double-precision)"))
  (`MaterialInstanceDynamic.SetScalarParameterValue` (`self.WindowMaterial`) "Opacity_Param" Opacity))

(fn `SetWindowDimensions`
  (params (Height :type "Float (double-precision)") (Width :type "Float (double-precision)"))
  (`SceneComponent.SetWorldScale3D` (`self.window`) (`KismetMathLibrary.MakeVector` (* Height 100.0) (* Width 100.0) 100.0)))

(fn `SetWindowPositionAndRotation`
  (params (Transform :type "Transform Structure"))
  (`self.K2_SetActorRelativeLocation` (`KismetMathLibrary.MakeVector` (.x (.location Transform)) (+ (.y (.location Transform)) 1.0) (.z (.location Transform))) false true)
  (`self.K2_SetActorRelativeRotation` (`KismetMathLibrary.MakeRotator` (+ (.roll (.rotation Transform)) 90.0) (+ (.pitch (.rotation Transform)) 90.0) (.yaw (.rotation Transform))) false true))

(fn `UserConstructionScript`)