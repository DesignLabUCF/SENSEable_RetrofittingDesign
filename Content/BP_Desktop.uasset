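; BP_Desktop constrains movement of the UXT input simulation actor, apparently for desktop play without a headset.
; Each Tick it scales that actor's movement since the last frame by VelocityMultiplier, clamps X and Y to a fixed box, then pins Z to standing or crouch height.
; The resulting location is saved for the next frame's scaling, and Caps Lock toggles the crouch state.
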(event `self.ReceiveTick`
  (params (DeltaSeconds :type "Float (single-precision)"))
  (`self.ConstrainVelocity`)
  (`self.ConstrainXandY`)
  (`self.ConstrainZ`)
  (bind _returnvalue (`GameplayStatics.GetActorOfClass` "/Script/UXToolsInputSimulation.UxtInputSimulationActor"))
  (set `self.lastLocation` (`SceneComponent.K2_GetComponentLocation` (`Actor.RootComponent` _returnvalue))))

(event `Key|CapsLock`
  (params (Key :type "Key Structure"))
  (:`Pressed`
    (bind _isa (`/Engine/EditorBlueprintResources/StandardMacros.FlipFlop`)
      (:`A`
        _)
      (:`B`
        _))
    (set `self.bCrouched` _isa)))

(fn `ConstrainVelocity`
  (bind _lastlocation (`self.lastLocation`))
  (bind _returnvalue (`GameplayStatics.GetActorOfClass` "/Script/UXToolsInputSimulation.UxtInputSimulationActor"))
  (bind _rootcomponent (`Actor.RootComponent` _returnvalue))
  (`SceneComponent.K2_SetWorldLocation` _rootcomponent (+ _lastlocation (* (- (`SceneComponent.K2_GetComponentLocation` _rootcomponent) _lastlocation) (`self.velocityMultiplier`))) false false))

(fn `ConstrainXandY`
  (bind _returnvalue (`GameplayStatics.GetActorOfClass` "/Script/UXToolsInputSimulation.UxtInputSimulationActor"))
  (bind _rootcomponent (`Actor.RootComponent` _returnvalue))
  (`SceneComponent.K2_SetWorldLocation` _rootcomponent (`KismetMathLibrary.MakeVector` (`KismetMathLibrary.FClamp` (.x (`SceneComponent.K2_GetComponentLocation` _rootcomponent)) -40.0 250.0) (`KismetMathLibrary.FClamp` (.y (`SceneComponent.K2_GetComponentLocation` _rootcomponent)) 100.0 250.0) (.z (`SceneComponent.K2_GetComponentLocation` _rootcomponent))) false false))

(fn `ConstrainZ`
  (bind _returnvalue (`GameplayStatics.GetActorOfClass` "/Script/UXToolsInputSimulation.UxtInputSimulationActor"))
  (if (`self.bCrouched`)
    (bind _rootcomponent (`Actor.RootComponent` _returnvalue))
    (bind _returnvalue_2 (`SceneComponent.K2_GetComponentLocation` _rootcomponent))
    (`SceneComponent.K2_SetWorldLocation` _rootcomponent (`KismetMathLibrary.MakeVector` (.x _returnvalue_2) (.y _returnvalue_2) (`self.crouchHeight`)) false false)
    (else
      (`SceneComponent.K2_SetWorldLocation` _rootcomponent (`KismetMathLibrary.MakeVector` (.x _returnvalue_2) (.y _returnvalue_2) (`self.standingHeight`)) false false))))

(fn `UserConstructionScript`)